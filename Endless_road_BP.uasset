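; Endless road segment actor that removes itself once the player pawn is far away and closes off behind the pawn.
; From BeginPlay, a one-second Delay loop measures the distance to player pawn 0 and destroys the actor beyond a fixed threshold.
; When a DefaultPawn stops overlapping the Box, that box switches to a blocking collision profile.
; Spawning of further segments is not handled here.
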(event OnComponentEndOverlap(Box)
  (params (OverlappedComponent :type Primitive%20Component%20Object%20Reference) (OtherActor :type Actor%20Object%20Reference) (OtherComp :type Primitive%20Component%20Object%20Reference) (OtherBodyIndex :type Integer))
  (Utilities|Casting|CastToDefaultPawn OtherActor)
  (Collision|SetCollisionProfileName (Variables|Default|GetBox) "Blockall" false :!class /Script/Engine.PrimitiveComponent))

(event EventBeginPlay
  (if (> (Math|Vector|VectorLength (- (Transformation|GetActorLocation (Game|Player|GetPlayerPawn 0)) (Transformation|GetActorLocation))) 2.5e+04) :!label _label
    (Actor|DestroyActor)
    (else
      (Utilities|FlowControl|Delay 1.0)
      (goto _label))))

(event Collision|EventActorBeginOverlap
  (params (OtherActor :type Actor%20Object%20Reference)))

(event EventTick
  (params (DeltaSeconds :type Float%20%28single-precision%29)))

(fn ConstructionScript)